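; Game mode for a Counter-Strike-style team round game, handling spawning, round wins and match resets for Counter-Terrorists and Terrorists.
; Players spawn at random team spawn points and are tracked by team in alive and dead maps.
; When a death empties a team, the other team scores and a winner announcement shows.
; After a delay, players respawn, or a team reaching the max score triggers level restart, score reset and player destruction.
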(event Custom|RequestSpawnPlayer
  (params (PlayerController :type PC%20Counter%20Strike%20Object%20Reference) (Team :type Actor%20Class%20Reference))
  (Default|SpawnPlayer PlayerController Team (select (== Team "/Game/BluePrints/Player/BP_CounterTerrorist.BP_CounterTerrorist_C") (Transformation|GetActorTransform (.OutItem (Utilities|Array|Random (Variables|Default|GetCounterTerroristSpawnPoints)))) (Transformation|GetActorTransform (.OutItem (Utilities|Array|Random (Variables|Default|GetTerroristSpawnPoints)))))))

(event Custom|AddToPlayersAliveMap
  (params (Player :type BP%20Player%20Base%20Object%20Reference%20%28by%20ref%29))
  (bind _playersdeath (Variables|Default|GetPlayersDeath))
  (if (.ReturnValue (Utilities|Map|Find _playersdeath Player))
    (Utilities|Map|Remove _playersdeath 0))
  (bind _playercontroller (Class|INTPlayerController|GetPlayerControllerRef(Message) (Pawn|GetController Player)))
  (Utilities|Map|Add (Variables|Default|GetPlayersAlive) Player (Variables|/Game/BluePrints/PC_CounterStrike.PC_CounterStrike_C|GetTeam _playercontroller)))

(event Custom|AddToPlayersDeathMap
  (params (Player :type BP%20Player%20Base%20Object%20Reference))
  (bind _playersalive (Variables|Default|GetPlayersAlive))
  (if (.ReturnValue (Utilities|Map|Find _playersalive Player))
    (Utilities|Map|Remove _playersalive Player))
  (bind _playercontroller (Class|INTPlayerController|GetPlayerControllerRef(Message) (Pawn|GetController Player)))
  (Utilities|Map|Add (Variables|Default|GetPlayersDeath) Player (Variables|/Game/BluePrints/PC_CounterStrike.PC_CounterStrike_C|GetTeam _playercontroller))
  (bind (_counterterroristalives _terroristalives) (Utilities|MCheckAmountOfLivingPlayers))
  (if (or (== _counterterroristalives 0) (== _terroristalives 0))
    (if (not (Variables|Default|GetbRoundOver))
      (CallFunction|FAddTeamScore)
      (for _array_element (Variables|Default|GetPlayersSpawned)
        (bind _playercontroller_2 (Class|INTPlayerController|GetPlayerControllerRef(Message) (Pawn|GetController _array_element)))
        (bind _values (Utilities|Map|Values (Variables|Default|GetPlayersAlive)))
        (Default|UpdateTeamWinAnnouncement _playercontroller_2 (Utilities|Array|Get(acopy) _values) (select (== (Utilities|Array|Get(acopy) _values) "/Game/BluePrints/Player/BP_CounterTerrorist.BP_CounterTerrorist_C") (Variables|Default|GetCounterTerroristScore) (Variables|Default|GetTerroristScore)) (Variables|Default|GetRespawnTimer))
        (Variables|Default|SetbRoundOver true))
      (Utilities|Map|Clear (Variables|Default|GetPlayersAlive))
      (Utilities|Map|Clear (Variables|Default|GetPlayersDeath))
      (Utilities|FlowControl|Delay (Variables|Default|GetRespawnTimer))
      (if (or (>= (Variables|Default|GetCounterTerroristScore) (Variables|Default|GetMaxScore)) (>= (Variables|Default|GetTerroristScore) (Variables|Default|GetMaxScore)))
        (for _array_element_2 (Variables|Default|GetPlayersSpawned)
          (Default|SRVRestartLevel _array_element_2))
        (Variables|Default|SetbRoundOver false)
        (Variables|Default|SetCounterTerroristScore 0)
        (Variables|Default|SetTerroristScore 0)
        (bind _outactors (Actor|GetAllActorsOfClass "/Game/BluePrints/Player/BP_PlayerBase.BP_PlayerBase_C"))
        (for _array_element_3 _outactors
          (Actor|DestroyActor _array_element_3))
        (else
          (for _array_element_4 (Variables|Default|GetPlayersSpawned)
            (Default|SRVAddtoPlayersAliveMap _array_element_4 _array_element_4)
            (Default|Respawn _array_element_4))
          (Variables|Default|SetbRoundOver false))))))

(event Custom|AddToPlayerSpawnArray
  (params (Player :type BP%20Player%20Base%20Object%20Reference))
  (bind _playersspawned (Variables|Default|GetPlayersSpawned))
  (Utilities|Array|SetArrayElem _playersspawned (Utilities|Array|Length _playersspawned) Player true))

(event EventPostLogin
  (params (NewPlayer :type Player%20Controller%20Object%20Reference))
  (Utilities|Array|Add (Variables|Default|GetConnectedPlayers) NewPlayer)
  (bind _outactors (Actor|GetAllActorsOfClass "/Game/BluePrints/SpanwPoint/BP_CounterTerrorisSpawnPoint.BP_CounterTerrorisSpawnPoint_C"))
  (Variables|Default|SetCounterTerroristSpawnPoints _outactors)
  (bind _outactors_2 (Actor|GetAllActorsOfClass "/Game/BluePrints/SpanwPoint/BP_TerrorisSpawnPoint.BP_TerrorisSpawnPoint_C"))
  (Variables|Default|SetTerroristSpawnPoints _outactors_2))

(fn ConstructionScript)

(fn FAddTeamScore
  (if (== (Variables|Default|GetCounterTerroristsAlive) 0)
    (Math|Integer|IncrementInt (Variables|Default|GetTerroristScore))
    (else
      (Math|Integer|IncrementInt (Variables|Default|GetCounterTerroristScore)))))

(fn GetGameModeRef
  (return self))